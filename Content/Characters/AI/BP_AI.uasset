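; BP_AI is an AI character that detects the player and performs a melee jab.
; Pawn sensing sets a "hasSeenPlayer?" blackboard flag when it sees BP_ThirdPersonCharacter; this graph never clears it.
; The AttackPlayer event sphere-traces forward for pawns, with debug drawing, and plays a left jab montage if it hits the player.
; The attack applies no damage here, and nothing in this file calls it.
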(event OnSeePawn(PawnSensing)
  (params (Pawn :type Pawn%20Object%20Reference))
  (Utilities|Casting|CastToBP_ThirdPersonCharacter Pawn)
  (AI|Components|Blackboard|SetValueasBool (AI|GetBlackboard (AI|GetAIController self)) (Utilities|Name|MakeLiteralName "hasSeenPlayer?") true))

(event Custom|AttackPlayer
  (bind _returnvalue (Transformation|GetActorLocation))
  (bind (_outhit _returnvalue_2) (Collision|SphereTraceForObjects _returnvalue (+ _returnvalue (* (Math|Vector|GetForwardVector (Transformation|GetActorRotation)) 2.5e+02)) 1.2e+02 (Utilities|Array|MakeArray "ObjectTypeQuery3") false 0 "ForDuration"))
  (if _returnvalue_2
    (Utilities|Casting|CastToBP_ThirdPersonCharacter (.HitActor (Collision|BreakHitResult _outhit)))
    (Animation|PlayAnimMontage "/Game/BoxingAssets/Boxing01/data/Source/FBX/Root_Motion/Box1_M3_Left_Jab_A_Anim_Montage.Box1_M3_Left_Jab_A_Anim_Montage" 1.0 "None")))

(event EventBeginPlay)

(event Collision|EventActorBeginOverlap
  (params (OtherActor :type Actor%20Object%20Reference)))

(event EventTick
  (params (DeltaSeconds :type Float%20%28single-precision%29)))

(fn ConstructionScript)