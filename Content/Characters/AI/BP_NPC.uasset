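; NPC character that chases the player and has boxing punch logic.
; Tick switches on a state fixed to Chase, so it calls AI MoveTo toward the player every frame and never reaches the Attack branch.
; HandleAIPunch plays a random jab or hook montage, re-arms itself by timer and immediately resets its DoOnce.
; AIPunch duplicates the random montage choice but is not called here.
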(event Custom|HandleAIPunch
  (Utilities|FlowControl|DoOnce false :!label _label
    (:Completed
      (switch int (Math|Random|RandomIntegerinRange 0 1)
        (:0
          (Animation|PlayAnimMontage "/Game/BoxingAssets/Boxing01/data/Source/FBX/Root_Motion/Box1_M3_Left_Jab_A_Anim_Montage.Box1_M3_Left_Jab_A_Anim_Montage" 1.0 "None")
          (Utilities|Time|SetTimerbyFunctionName 0 "HandleAIPunch" 1e+02)
          (goto _label Reset))
        (:1
          (Animation|PlayAnimMontage "/Game/BoxingAssets/Boxing01/data/Source/FBX/Root_Motion/Box1_M3_Right_Hook_Anim_Montage.Box1_M3_Right_Hook_Anim_Montage" 1.0 "None")
          (Utilities|Time|SetTimerbyFunctionName 0 "HandleAIPunch" 1e+02)
          (goto _label Reset))))))

(event EventBeginPlay
  (Variables|Default|SetTargetPlayer (Game|GetPlayerCharacter 0)))

(event EventTick
  (params (DeltaSeconds :type Float%20%28single-precision%29))
  (switch Utilities|FlowControl|Switch|SwitchonAIStateEnum "NewEnumerator0"
    (:NewEnumerator0
      (AI|AIMoveTo self "0, 0, 0" (Game|GetPlayerCharacter 0) 5.0 false))
    (:NewEnumerator1
      (CallFunction|HandleAIPunch))))

(fn ConstructionScript)

(fn AIPunch
  (switch int (Math|Random|RandomIntegerinRange 0 1)
    (:0
      (Animation|PlayAnimMontage "/Game/BoxingAssets/Boxing01/data/Source/FBX/Root_Motion/Box1_M3_Left_Jab_A_Anim_Montage.Box1_M3_Left_Jab_A_Anim_Montage" 1.0 "None"))
    (:1
      (Animation|PlayAnimMontage "/Game/BoxingAssets/Boxing01/data/Source/FBX/Root_Motion/Box1_M3_Right_Hook_Anim_Montage.Box1_M3_Right_Hook_Anim_Montage" 1.0 "None"))))